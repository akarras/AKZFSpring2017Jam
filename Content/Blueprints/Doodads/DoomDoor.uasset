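; DoomDoor is the level-ending door that opens only when the player holds Pizza, Beer and Donut.
; Box overlap with SpringyCharacter enables input and shows an EToUse prompt listing NeededPickups.
; Use subtracts the GameInstance's CurrentPickups from that list, resetting it if any remain.
; On success it consumes the items, shatters AkDoorDM with physics and radius damage, then after a delay destroys itself and shows YouWin.
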(event `DestroyDoor`
  (bind _ak_door_dm (`self.ak_door_DM`))
  (`ActorComponent.K2_DestroyComponent` (`self.Beer`) :!label _label)
  (`ActorComponent.K2_DestroyComponent` (`self.Donut`))
  (`ActorComponent.K2_DestroyComponent` (`self.Pizza`))
  (`PrimitiveComponent.SetSimulatePhysics` _ak_door_dm true)
  (`DestructibleComponent.ApplyRadiusDamage` _ak_door_dm 100.0 (`SceneComponent.K2_GetComponentLocation` _ak_door_dm) 100.0 200.0 true)
  (`KismetSystemLibrary.Delay` 5.0)
  (`self.K2_DestroyActor`)
  (bind _returnvalue (`|CreateWidget` "/Game/Blueprints/UI/YouWin.YouWin_C"))
  (`UserWidget.AddToViewport` _returnvalue 0))

(event `InputAction|Use`
  (params (Key :type "Key Structure" :default "AnyKey"))
  (:`Pressed`
    (bind _asspring_game_instance (cast `/Game/Blueprints/Game/Spring_GameInstance` (`GameplayStatics.GetGameInstance`)))
    (bind _currentpickups (`/Game/Blueprints/Game/Spring_GameInstance.CurrentPickups` _asspring_game_instance))
    (for _array_element _currentpickups
      (`KismetArrayLibrary.Array_RemoveItem` (`self.neededPickups`) _array_element))
    (if (== (`KismetArrayLibrary.Array_Length` (`self.neededPickups`)) 0)
      (`KismetArrayLibrary.Array_RemoveItem` _currentpickups "Pizza")
      (`KismetArrayLibrary.Array_RemoveItem` _currentpickups "Beer")
      (`KismetArrayLibrary.Array_RemoveItem` _currentpickups "Donut")
      (goto _label)
      (else
        (`self.CleanArray`)))))

(event `SetFound`
  (params (Pickup :type "StaticMeshComponent Object Reference")))

(event `self.Box.OnComponentBeginOverlap`
  (params (OverlappedComponent :type "PrimitiveComponent Object Reference") (OtherActor :type "Actor Object Reference") (OtherComp :type "PrimitiveComponent Object Reference") (OtherBodyIndex :type Integer) (bFromSweep :type Boolean) (SweepResult :type "HitResult Structure (by ref)"))
  (cast `/Game/Blueprints/Player/SpringyCharacter` OtherActor)
  (`self.EnableInput` (`GameplayStatics.GetPlayerController` 0))
  (bind _returnvalue (`|CreateWidget` "/Game/Blueprints/UI/EToUse.EToUse_C"))
  (bind _output_get (set `self.EToUse` _returnvalue))
  (`UserWidget.AddToViewport` _output_get 0)
  (`TextBlock.SetText` (`/Game/Blueprints/UI/EToUse.Description` _returnvalue) (`|FormatText` "You still need: {items}" (`KismetTextLibrary.Conv_StringToText` (`KismetStringLibrary.JoinStringArray` (`self.neededPickups`) ", ")))))

(event `self.Box.OnComponentEndOverlap`
  (params (OverlappedComponent :type "PrimitiveComponent Object Reference") (OtherActor :type "Actor Object Reference") (OtherComp :type "PrimitiveComponent Object Reference") (OtherBodyIndex :type Integer))
  (cast `/Game/Blueprints/Player/SpringyCharacter` OtherActor)
  (`self.DisableInput` (`GameplayStatics.GetPlayerController` 0))
  (`Widget.RemoveFromParent` (`self.EToUse`)))

(fn `AddItem`
  (params (Pickup :type String))
  (`KismetArrayLibrary.Array_Add` (`self.neededPickups`) Pickup))

(fn `CleanArray`
  (`KismetArrayLibrary.Array_Clear` (`self.neededPickups`))
  (`self.AddItem` "Pizza")
  (`self.AddItem` "Beer")
  (`self.AddItem` "Donut"))

(fn `UserConstructionScript`)