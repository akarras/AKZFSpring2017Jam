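; Enemy Behavior Tree tick node, likely a service, that keeps a Blackboard target set to a SpringyCharacter within CheckDistance.
; Each tick it clears an existing target that is out of range, using the LengthCheck distance helper.
; With no valid target, it scans all SpringyCharacter actors and stores those in range without breaking, so the last match wins rather than the nearest.
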(event `self.ReceiveTick`
  (params (OwnerActor :type "Actor Object Reference") (DeltaSeconds :type "Float (single-precision)"))
  (bind _returnvalue (`BTFunctionLibrary.GetBlackboardValueAsActor` (`self.TargetKey`)))
  (`/Engine/EditorBlueprintResources/StandardMacros.IsValid` _returnvalue
    (:`Is Valid`
      (bind _returnvalue_2 (`self.LengthCheck` OwnerActor _returnvalue))
      (if (not _returnvalue_2)
        (`BTFunctionLibrary.ClearBlackboardValue` (`self.TargetKey`))))
    (:`Is Not Valid`
      (bind _outactors (`GameplayStatics.GetAllActorsOfClass` "/Game/Blueprints/Player/SpringyCharacter.SpringyCharacter_C"))
      (for _array_element _outactors
        (bind _returnvalue_3 (`self.LengthCheck` OwnerActor _array_element))
        (if _returnvalue_3
          (`BTFunctionLibrary.SetBlackboardValueAsObject` (`self.TargetKey`) _array_element))))))

(fn `LengthCheck`
  (params (self2 :type "Actor Object Reference") (self3 :type "Actor Object Reference"))
  (returns (ReturnValue :type Boolean))
  (return (<= (`KismetMathLibrary.VSize` (- (`Actor.K2_GetActorLocation` self3) (`Actor.K2_GetActorLocation` self2))) (`self.CheckDistance`))))