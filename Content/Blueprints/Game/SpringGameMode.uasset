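; SpringGameMode is a game mode that chooses the player's spawn point based on the level they came from.
; Its FindPlayerStart override turns LastWorld from Spring_GameInstance into a tag and returns the first actor carrying it.
; If no actor has that tag, it falls back to the first PlayerStart found in the level.
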(fn `FindPlayerStart`
  (params (Player :type "Controller Object Reference") (IncomingName :type String))
  (returns (ReturnValue :type "Actor Object Reference"))
  (bind _asspring_game_instance (cast `/Game/Blueprints/Game/Spring_GameInstance` (`GameplayStatics.GetGameInstance`)))
  (bind _outactors (`GameplayStatics.GetAllActorsWithTag` (`KismetStringLibrary.Conv_StringToName` (`/Game/Blueprints/Game/Spring_GameInstance.LastWorld` _asspring_game_instance))))
  (if (> (`KismetArrayLibrary.Array_Length` _outactors) 0)
    (return (`KismetArrayLibrary.Array_Get` _outactors))
    (else
      (bind _outactors_2 (`GameplayStatics.GetAllActorsOfClass` "/Script/Engine.PlayerStart"))
      (return (`KismetArrayLibrary.Array_Get` _outactors_2)))))

(fn `UserConstructionScript`)