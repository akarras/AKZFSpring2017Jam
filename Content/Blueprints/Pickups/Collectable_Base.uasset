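; Base pickup actor that spins in place and is collected when the player's SpringyCharacter touches it.
; Tick yaws the actor by RotationSpeed scaled by delta time.
; The Sphere overlap adds the pickup's Type to the Spring_GameInstance, then destroys the actor.
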(event `self.ReceiveBeginPlay`)

(event `self.ReceiveTick`
  (params (DeltaSeconds :type "Float (single-precision)"))
  (`self.K2_AddActorLocalRotation` (`KismetMathLibrary.MakeRotator` 0.0 0.0 (* DeltaSeconds (`self.RotationSpeed`))) false true))

(event `self.Sphere.OnComponentBeginOverlap`
  (params (OverlappedComponent :type "PrimitiveComponent Object Reference") (OtherActor :type "Actor Object Reference") (OtherComp :type "PrimitiveComponent Object Reference") (OtherBodyIndex :type Integer) (bFromSweep :type Boolean) (SweepResult :type "HitResult Structure (by ref)"))
  (cast `/Game/Blueprints/Player/SpringyCharacter` OtherActor)
  (bind _asspring_game_instance (cast `/Game/Blueprints/Game/Spring_GameInstance` (`GameplayStatics.GetGameInstance`)))
  (`/Game/Blueprints/Game/Spring_GameInstance.AddPickup` _asspring_game_instance (`self.Type`))
  (`self.K2_DestroyActor`))

(fn `UserConstructionScript`)