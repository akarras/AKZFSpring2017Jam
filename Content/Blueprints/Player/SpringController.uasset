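; SpringController is a player controller that handles pausing the game with an escape menu.
; Pause input creates an EscapeMenu widget, pauses the game and shows the mouse cursor, or reverses this when already paused.
; A ResumePlay event shares the same unpause path, which removes all widgets and hides the cursor.
; All widgets are also cleared on BeginPlay.
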(event `self.ReceiveBeginPlay`
  (`WidgetLayoutLibrary.RemoveAllWidgets`))

(event `InputAction|Pause`
  (params (Key :type "Key Structure" :default "AnyKey"))
  (:`Pressed`
    (if (`GameplayStatics.IsGamePaused`)
      (`WidgetLayoutLibrary.RemoveAllWidgets` :!label _label)
      (`GameplayStatics.SetGamePaused` false)
      (set `self.bShowMouseCursor` false)
      (else
        (bind _returnvalue (`|CreateWidget` "/Game/Blueprints/UI/EscapeMenu.EscapeMenu_C"))
        (bind _output_get (set `self.Widget` _returnvalue))
        (`UserWidget.AddToViewport` _output_get 0)
        (`GameplayStatics.SetGamePaused` true)
        (set `self.bShowMouseCursor` true)))))

(event `Resume Play`
  (goto _label))

(fn `UserConstructionScript`)